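; Test dice actor Blueprint that displays a debug readout of whether the die is rolling.
; Each Tick writes the result of IsRolling, which is not defined in this graph, into the IsRollingText component.
; The text is moved to a fixed height above Mesh with its world rotation zeroed, so it stays upright regardless of the die's orientation.
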(event `self.ReceiveTick`
  (params (DeltaSeconds :type "Float (single-precision)"))
  (`TextRenderComponent.K2_SetText` (`self.IsRollingText`) (`KismetTextLibrary.Conv_StringToText` (`KismetStringLibrary.Concat_StrStr` "Is rolling: " (`KismetStringLibrary.Conv_BoolToString` (`self.isRolling`)))))
  (`SceneComponent.K2_SetWorldLocation` (`self.IsRollingText`) (+ (`SceneComponent.K2_GetComponentLocation` (`self.Mesh`)) (0.0 0.0 100.0)) false false)
  (`SceneComponent.K2_SetWorldRotation` :`self` (`self.IsRollingText`)))

(fn `UserConstructionScript`)